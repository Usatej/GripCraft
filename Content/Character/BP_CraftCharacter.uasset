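; Player character for a block-based crafting game that handles mining, item use and item switching.
; InventoryComponent drives the held item mesh, and an input axis cycles the selection with wraparound.
; Primary action swings an equipped tool through HitTimeline, whose event triggers MiningComponent hits, while Tick eases the rotation back; secondary action uses usable items.
; X sets the block found by a camera trace, nudged along the hit normal, to air.
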(event EventTick
  (params (DeltaSeconds :type Float%20%28single-precision%29))
  ;[1 1 1] Primary action
  (if (not (Variables|Default|GetbHitting))
    (Transformation|SetRelativeRotation (Variables|Default|GetSelectedItemMeshComponent) (Math|Interpolation|RInterpTo (Variables|/Script/Engine.SceneComponent|GetRelativeRotation (Variables|Default|GetSelectedItemMeshComponent)) (Variables|Default|GetSelectedItemStartRotation) DeltaSeconds 15.0) false false)))

(event EventBeginPlay
  (Variables|Default|SetSelectedItemStartRotation (Variables|/Script/Engine.SceneComponent|GetRelativeRotation (Variables|Default|GetSelectedItemMeshComponent)))
  (EventDispatchers|BindEventtoOnSelectedItemChanged (Variables|Default|GetInventoryComponent) (EventDispatchers|CreateEvent :!event OnSelectedItemChanged))
  (Class|CraftInventoryComponent|SelectItembyIndex (Variables|Default|GetInventoryComponent)))

(event Input|ActionEvents|InputActionPrimaryAction
  (params (Key :type Key%20Structure :default "None"))
  ;[1 1 1] Primary action
  (:Pressed
    (Utilities|HasToolEquiped
      (:Yes
        (Variables|Default|SetbHitting true)
        (bind _rotationalpha (Timeline|HitTimeline PlayFromStart)
          (:Update
            (CallFunction|UpdateSelectedItemRotation _rotationalpha))
          (:HitEvent
            (Class|CraftMiningComponent|TryHitBlockinFrontOf (Variables|Default|GetMiningComponent)))))))
  (:Released
    (Variables|Default|SetbHitting false)
    (Timeline|HitTimeline Stop)))

(event Input|ActionEvents|InputActionSecondaryAction
  (params (Key :type Key%20Structure :default "None"))
  (bind _inventorycomponent (Variables|Default|GetInventoryComponent))
  (bind _returnvalue (Class|CraftInventoryComponent|GetSelectedItem _inventorycomponent))
  (:Pressed
    (Utilities|IsValid _returnvalue
      (:Is%20Valid
        (if (Class|CraftItem|HasTag _returnvalue "(TagName=\"Item.Usable\")")
          (bind _ascraft_item_usable (Utilities|Casting|CastToCraftItemUsable _returnvalue))
          (Class|CraftItemUsable|Use _ascraft_item_usable self))))))

(event Input|AxisEvents|InputAxisChangeItem
  (params (AxisValue :type Float%20%28single-precision%29))
  (CallFunction|ChangeItem AxisValue))

(event Input|KeyboardEvents|X
  (params (Key :type Key%20Structure :default "None"))
  (:Pressed
    (bind (_success _location) (CallFunction|TraceforBlock false))
    (if _success
      (Class|CraftWorldSubsystem|SetBlockBP (Subsystems|GetCraftWorldSubsystem) (Class|CraftCoordsUtils|ConvertWorldPositiontoWorldCoords _location) "(TagName=\"Block.Air\")" true))))

(fn ConstructionScript)

(fn TraceforBlock
  (params (AddNormal :type Boolean))
  (bind _returnvalue (Game|GetPlayerCameraManager 0))
  (bind _returnvalue_2 (Camera|GetCameraLocation _returnvalue))
  (bind (_outhit _returnvalue_3) (Collision|LineTraceByChannel _returnvalue_2 (+ _returnvalue_2 (* (Math|Vector|GetForwardVector (Camera|GetCameraRotation _returnvalue)) "800.000000,800.000000,800.000000")) "TraceTypeQuery1" false 0 "None"))
  (if _returnvalue_3
    (if AddNormal
      (return true (Class|CraftCoordsUtils|AlignWorldPosition (+ (.Location (Collision|BreakHitResult _outhit)) (.Normal (Collision|BreakHitResult _outhit)))))
      (else
        (return true (Class|CraftCoordsUtils|AlignWorldPosition (- (.Location (Collision|BreakHitResult _outhit)) (.Normal (Collision|BreakHitResult _outhit)))))))
    (else
      (return false "0, 0, 0"))))

(fn UpdateSelectedItemRotation
  (params (LerpValue :type Float%20%28double-precision%29))
  (Transformation|SetRelativeRotation (Variables|Default|GetSelectedItemMeshComponent) (Math|Rotator|Lerp(Rotator) (Variables|Default|GetSelectedItemStartRotation) (Variables|Default|GetSelectedItemEndRotation) LerpValue) false false))

(fn OnSelectedItemChanged
  (params (Item :type Craft%20Item%20Object%20Reference))
  (Utilities|IsValid Item
    (:Is%20Valid
      (Components|StaticMesh|SetStaticMesh (Variables|Default|GetSelectedItemMeshComponent) (Variables|/Script/Gripcraft.CraftItem|GetMesh Item)))
    (:Is%20Not%20Valid
      (Components|StaticMesh|SetStaticMesh (Variables|Default|GetSelectedItemMeshComponent) 0))))

(fn ChangeItem
  (params (AxisValue :type Float%20%28double-precision%29))
  (if (> (Math|Float|Absolute(Float) AxisValue) 0.9)
    (LocalVariables|SetSelectedItemIndex (Class|CraftInventoryComponent|GetSelectedItemIndex (Variables|Default|GetInventoryComponent)))
    (if (>= AxisValue 0.0)
      (Math|Integer|IncrementInt (LocalVariables|GetSelectedItemIndex)
        (:%20%20
          _))
      (else
        (Math|Integer|DecrementInt (LocalVariables|GetSelectedItemIndex)
          (:%20%20
            _))))
    (if (< (LocalVariables|GetSelectedItemIndex) 0)
      (LocalVariables|SetSelectedItemIndex (+ (LocalVariables|GetSelectedItemIndex) (Utilities|Array|Length (Class|CraftInventoryComponent|GetItems (Variables|Default|GetInventoryComponent))))))
    (Class|CraftInventoryComponent|SelectItembyIndex (Variables|Default|GetInventoryComponent) (Math|Integer|%(Integer) (LocalVariables|GetSelectedItemIndex) (Utilities|Array|Length (Class|CraftInventoryComponent|GetItems (Variables|Default|GetInventoryComponent)))))))