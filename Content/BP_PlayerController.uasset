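; Player controller Blueprint that toggles the game menu and debug info display through BP_HUD.
; It starts in game-only input mode, and each GameMenu press flips menu visibility, switching between Game and UI input with a visible cursor and game-only input with a hidden cursor.
; Each DebugMenu press flips debug info visibility on the HUD without changing input mode.
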(event EventBeginPlay
  (Input|SetInputModeGameOnly self))

(event Input|ActionEvents|InputActionDebugMenu
  (params (Key :type Key%20Structure :default "None"))
  (:Pressed
    (bind _asbp_hud (Utilities|Casting|CastToBP_HUD (HUD|GetHUD)))
    (bind _isa (Utilities|FlowControl|FlipFlop)
      (:A
        _)
      (:B
        _))
    (Default|SetDebugInfoVisibiltiy _asbp_hud _isa)))

(event Input|ActionEvents|InputActionGameMenu
  (params (Key :type Key%20Structure :default "None"))
  (bind _returnvalue (Game|GetPlayerController 0))
  (bind _returnvalue_2 (Game|GetPlayerController 0))
  (:Pressed
    (bind _asbp_hud (Utilities|Casting|CastToBP_HUD (HUD|GetHUD)))
    (bind _isa (Utilities|FlowControl|FlipFlop)
      (:A
        _)
      (:B
        _))
    (Default|SetGameMenuVisibility _asbp_hud _isa)
    (if _isa
      (Input|SetInputModeGameandUI _returnvalue_2 0 "DoNotLock" false)
      (Variables|/Script/Engine.PlayerController|SetbShowMouseCursor _returnvalue_2 true)
      (else
        (Input|SetInputModeGameOnly _returnvalue)
        (Variables|/Script/Engine.PlayerController|SetbShowMouseCursor _returnvalue false)))))

(fn ConstructionScript)